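; Puzzle text actor, apparently a readable stone, that displays one of its stored texts on screen.
; A sphere overlap with the third-person character enables input on the actor, and leaving disables it and removes the widget.
; The TextStone event uses a FlipFlop to create a WBP_TextDoor widget with the text selected by TextIndex, or remove it.
; Leaving the sphere does not reset that FlipFlop.
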(event OnComponentBeginOverlap(Sphere)
  (params (OverlappedComponent :type Primitive%20Component%20Object%20Reference) (OtherActor :type Actor%20Object%20Reference) (OtherComp :type Primitive%20Component%20Object%20Reference) (OtherBodyIndex :type Integer) (bFromSweep :type Boolean) (SweepResult :type Hit%20Result%20Structure%20%28by%20ref%29))
  ;[0.15 0.15 0.15 0.5] Appel BP chara
  (Utilities|Casting|CastToBP_ThirdPersonCharacter OtherActor)
  (Input|EnableInput (Game|GetPlayerController 0)))

(event OnComponentEndOverlap(Sphere)
  (params (OverlappedComponent :type Primitive%20Component%20Object%20Reference) (OtherActor :type Actor%20Object%20Reference) (OtherComp :type Primitive%20Component%20Object%20Reference) (OtherBodyIndex :type Integer))
  ;[0.15 0.15 0.15 0.5] Appel BP chara
  (Utilities|Casting|CastToBP_ThirdPersonCharacter OtherActor)
  (Input|DisableInput (Game|GetPlayerController 0))
  (Widget|RemovefromParent (Variables|Default|GetTextWBP)))

(event EventTextStone
  ;[0.15 0.15 0.15 0.5] Affichage text
  (Utilities|FlowControl|FlipFlop
    (:A
      (bind _returnvalue (UserInterface|CreateWidget "/Game/Civilisation_perdue/Gameplay/Enigme/WBP_TextDoor.WBP_TextDoor_C"))
      (bind _output_get (Variables|Default|SetTextWBP _returnvalue))
      (UserInterface|Viewport|AddtoViewport _output_get 0)
      (Rendering|Components|TextRender|SetText (Variables|/Game/Civilisation_perdue/Gameplay/Enigme/WBP_TextDoor.WBP_TextDoor_C|GetTextBlock (Variables|Default|GetTextWBP)) (Utilities|Text|ToText(String) (Utilities|Array|Get(acopy) (Variables|Default|GetText) (Variables|Default|GetTextIndex)))))
    (:B
      (Widget|RemovefromParent (Variables|Default|GetTextWBP)))))

(fn ConstructionScript)