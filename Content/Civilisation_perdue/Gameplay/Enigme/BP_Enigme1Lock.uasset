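; Rotating cube lock for the first puzzle (Enigme 1) that advances to its next face on each player interaction.
; Six face components supply the relative rotations, and the current index wraps back to the first after the last.
; Interaction plays an animation that lerps the cube along the shortest path between faces, ignoring input until it finishes and the index increments.
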(event EventBeginPlay)

(event EventInteractionPlayer
  (if (not (Variables|Default|GetAnimationPlaying))
    (CallFunction|SetTargetRotation)
    (CallFunction|AnimPlayfromStart)
    (Variables|Default|SetAnimationPlaying true)))

(event EventAnimUpdate
  (params (ValueAnim :type Float%20%28double-precision%29))
  (Transformation|SetRelativeRotation (Variables|Default|GetCube) (Math|Rotator|Lerp(Rotator) (Variables|Default|GetStartRotation) (Variables|Default|GetEndRotation) ValueAnim true) false false))

(event EventAnimFinish
  (Variables|Default|SetCurrentIndex (select (> (+ (Variables|Default|GetCurrentIndex) 1) (Utilities|Array|LastIndex (CallFunction|GetList))) 0 (+ (Variables|Default|GetCurrentIndex) 1)))
  (Variables|Default|SetAnimationPlaying false))

(fn ConstructionScript
  (|CallParentFunction))

(fn SetTargetRotation
  (bind _currentindex (Variables|Default|GetCurrentIndex))
  (bind _returnvalue (+ _currentindex 1))
  (Variables|Default|SetStartRotation (Variables|/Script/Engine.SceneComponent|GetRelativeRotation (CallFunction|GetListeFaceCube (Variables|Default|GetCurrentIndex))))
  (Variables|Default|SetEndRotation (Variables|/Script/Engine.SceneComponent|GetRelativeRotation (CallFunction|GetListeFaceCube (select (> _returnvalue (Utilities|Array|LastIndex (CallFunction|GetList))) 0 _returnvalue)))))

(fn GetListeFaceCube
  (params (Index :type Integer))
  (return (Utilities|Array|Get(acopy) (CallFunction|GetList) Index)))

(fn GetList
  (return (Utilities|Array|MakeArray (Variables|Default|Get01) (Variables|Default|Get02) (Variables|Default|Get03) (Variables|Default|Get04) (Variables|Default|Get05) (Variables|Default|Get06))))