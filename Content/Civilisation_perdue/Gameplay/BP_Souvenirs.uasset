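; BP_Souvenirs is a memory ("souvenir") Blueprint that shows a sequence of dialogue lines through a Talk event.
; Overlapping its Box shows a WBP_DialPressE prompt while lines remain, and ending the overlap removes it.
; Each Talk call increments TalkIndex, removes the prompt, and displays that Dialogue entry in a lazily created WP_Dialogue widget.
; Once TalkIndex reaches EndNumber, Talk removes both widgets and the prompt stops appearing.
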(event OnComponentBeginOverlap(Box)
  (params (OverlappedComponent :type Primitive%20Component%20Object%20Reference) (OtherActor :type Actor%20Object%20Reference) (OtherComp :type Primitive%20Component%20Object%20Reference) (OtherBodyIndex :type Integer) (bFromSweep :type Boolean) (SweepResult :type Hit%20Result%20Structure%20%28by%20ref%29))
  ;[0.15 0.15 0.15 0.5] Affichage Press E
  (if (< (Variables|Default|GettalkIndex) (Variables|Default|GetEndNumber))
    (bind _returnvalue (UserInterface|CreateWidget "/Game/Civilisation_perdue/Gameplay/WBP_DialPressE.WBP_DialPressE_C"))
    (bind _output_get (Variables|Default|SetDial _returnvalue))
    (UserInterface|Viewport|AddtoViewport _output_get 0)))

(event OnComponentEndOverlap(Box)
  (params (OverlappedComponent :type Primitive%20Component%20Object%20Reference) (OtherActor :type Actor%20Object%20Reference) (OtherComp :type Primitive%20Component%20Object%20Reference) (OtherBodyIndex :type Integer))
  ;[0.15 0.15 0.15 0.5] Affichage Press E
  (Widget|RemovefromParent (Variables|Default|GetDial)))

(event EventTalk
  ;[0.15 0.15 0.15 0.5] Dialogue
  (Math|Integer|IncrementInt (Variables|Default|GettalkIndex)
    (:%20%20
      (if (< (Variables|Default|GettalkIndex) (Variables|Default|GetEndNumber))
        (Widget|RemovefromParent (Variables|Default|GetDial))
        (Variables|Default|GetUI
          (:then
            _)
          (:else
            (bind _returnvalue (UserInterface|CreateWidget "/Game/Civilisation_perdue/Gameplay/WP_Dialogue.WP_Dialogue_C" (Game|GetPlayerController 0)))
            (bind _output_get (Variables|Default|SetUI _returnvalue))
            (UserInterface|Viewport|AddtoViewport _output_get 0)))
        (Rendering|Components|TextRender|SetText (Variables|/Game/Civilisation_perdue/Gameplay/WP_Dialogue.WP_Dialogue_C|GetTalkText (Variables|Default|GetUI)) (Utilities|Text|ToText(String) (Utilities|Array|Get(acopy) (Variables|Default|Getdialogue) (Variables|Default|GettalkIndex))))
        (else
          (Widget|RemovefromParent (Variables|Default|GetUI)))))))

(fn ConstructionScript)