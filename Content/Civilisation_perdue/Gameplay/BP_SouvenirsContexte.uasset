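; BP_SouvenirsContexte is a trigger that shows a line of contextual dialogue when something enters its sphere.
; On the first sphere overlap only, it creates a WP_Dialogue widget and fills its TalkText with the DialogueContexte entry at Index.
; The widget stays on screen for four seconds, then is removed from the viewport.
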(event OnComponentBeginOverlap(Sphere)
  (params (OverlappedComponent :type Primitive%20Component%20Object%20Reference) (OtherActor :type Actor%20Object%20Reference) (OtherComp :type Primitive%20Component%20Object%20Reference) (OtherBodyIndex :type Integer) (bFromSweep :type Boolean) (SweepResult :type Hit%20Result%20Structure%20%28by%20ref%29))
  (Utilities|FlowControl|DoOnce false
    (:Completed
      (bind _returnvalue (UserInterface|CreateWidget "/Game/Civilisation_perdue/Gameplay/WP_Dialogue.WP_Dialogue_C"))
      (bind _output_get (Variables|Default|SetDialContexte _returnvalue))
      (UserInterface|Viewport|AddtoViewport _output_get 0)
      (Variables|/Script/UMG.TextBlock|SetText (Variables|/Game/Civilisation_perdue/Gameplay/WP_Dialogue.WP_Dialogue_C|GetTalkText (Variables|Default|GetDialContexte)) (Utilities|Text|ToText(String) (Utilities|Array|Get(acopy) (Variables|Default|GetDialogueContexte) (Variables|Default|GetIndex))))
      (Utilities|FlowControl|Delay 4.0)
      (Widget|RemovefromParent (Variables|Default|GetDialContexte)))))

(fn ConstructionScript)