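; Puzzle door for the first enigma that unlocks when every cube in the LockCube map holds its expected index.
; On player interaction while locked, it compares each cube's CurrentIndex to the map value, opening on a full match or playing a closed-door animation on mismatches.
; Once unlocked, a FlipFlop alternates closing and opening.
; Both animations drive the Scene component's yaw through update events.
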(event EventAnimCloseUpdate
  (params (Value%20Anim :type Float%20%28double-precision%29))
  (Transformation|SetRelativeRotation (Variables|Default|GetScene) (Math|Rotator|MakeRotator 0.0 0.0 Value%20Anim) false false))

(event EventAnimUpdate
  (params (ValueAnim :type Float%20%28double-precision%29))
  (Transformation|SetRelativeRotation (Variables|Default|GetScene) (Math|Rotator|MakeRotator 0.0 0.0 ValueAnim) false false))

(event EventInteractionPlayer
  ;[0.15 0.15 0.15 0.5] Anim Porte (lock ou unlock)
  (if (Variables|Default|GetUnlock)
    (Utilities|FlowControl|FlipFlop
      (:A
        (Development|PrintString "Close")
        (CallFunction|AnimReverse))
      (:B
        (Development|PrintString "Open")
        (CallFunction|AnimPlayfromStart)))
    (else
      (Variables|Default|Setcach true)
      (bind _keys (Utilities|Map|Keys (Variables|Default|GetLockCube)))
      (for _array_element _keys
        (if (not (== (Variables|/Game/Civilisation_perdue/Dialogue/Enigme/BP_Enigme1Lock.BP_Enigme1Lock_C|GetCurrentIndex _array_element) (.Value (Utilities|Map|Find (Variables|Default|GetLockCube) _array_element))))
          (Variables|Default|Setcach false)
          (Development|PrintString "Porte close")
          (CallFunction|AnimClosePlayfromStart)))
      (if (Variables|Default|Getcach)
        (CallFunction|AnimPlay)
        (Variables|Default|SetUnlock true)))))

(fn ConstructionScript
  (|CallParentFunction))