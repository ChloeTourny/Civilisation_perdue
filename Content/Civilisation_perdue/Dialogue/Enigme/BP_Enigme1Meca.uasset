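; BP_Enigme1Meca is a puzzle mechanism actor, apparently a base for animated pieces of the first enigma.
; A timeline, its play rate set from DurationAnim at BeginPlay, can be played, restarted or reversed.
; Its Percent track samples CurveAnim, scaled by ValueAnim, to feed an update event, and completion calls AnimFinish.
; The update, finish and player interaction events are empty hooks, so no concrete motion is defined here.
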(event EventBeginPlay)

(event Collision|EventActorBeginOverlap
  (params (OtherActor :type Actor%20Object%20Reference)))

(event EventTick
  (params (DeltaSeconds :type Float%20%28single-precision%29)))

(event Custom|AnimGraph_BeginPlay
  (Components|Timeline|SetPlayRate (Variables|Default|GetAnimationTimeline) (/ 1.0 (Variables|Default|GetDurationAnim))))

(event Custom|Anim_Play
  (bind _percent (Timeline|AnimationTimeline Play)
    (:Update
      (CallFunction|AnimUpdate (* (Math|Curves|GetFloatValue (Variables|Default|GetCurveAnim) _percent) (Variables|Default|GetValueAnim))))
    (:Finished
      (CallFunction|AnimFinish))))

(event Custom|Anim_PlayFromStart
  (bind _percent (Timeline|AnimationTimeline PlayFromStart)
    (:Update
      (CallFunction|AnimUpdate (* (Math|Curves|GetFloatValue (Variables|Default|GetCurveAnim) _percent) (Variables|Default|GetValueAnim))))
    (:Finished
      (CallFunction|AnimFinish))))

(event Custom|Anim_Update
  (params (ValueAnim :type Float%20%28double-precision%29)))

(event Custom|AnimFinish)

(event Custom|InteractionPlayer)

(event Custom|Anim_Reverse
  (bind _percent (Timeline|AnimationTimeline Reverse)
    (:Update
      (CallFunction|AnimUpdate (* (Math|Curves|GetFloatValue (Variables|Default|GetCurveAnim) _percent) (Variables|Default|GetValueAnim))))
    (:Finished
      (CallFunction|AnimFinish))))

(fn ConstructionScript)